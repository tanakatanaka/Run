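; BP_Map is a cleanable surface that paints where the player is and measures how much dirt or blood has been cleaned.
; BeginPlay duplicates the origin render targets and creates dynamic materials for dirt, blood and calculation.
; CleanPaint converts player position to plane UV via bounds, then draws the dirt material into the texture target.
; CheckCleanPer then draws the calculation material into a percent target and prints its cleaning rate.
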(event `self.ReceiveBeginPlay`
  (`|ExecutionSequence`
    (:`then_0`
      (bind _returnvalue (`KismetMaterialLibrary.CreateDynamicMaterialInstance` "/Game/Texture/M_DirtCurrent.M_DirtCurrent"))
      (set `self.dartMat` _returnvalue)
      (`KismetRenderingLibrary.ClearRenderTarget2D` (`self.new_TextureRenderTarget`) (struct :`R` 1.0 :`G` 1.0 :`B` 1.0))
      (`KismetRenderingLibrary.ClearRenderTarget2D` (`self.new_Percent Render Target`) (struct :`R` 1.0 :`G` 1.0 :`B` 1.0))
      (bind _returnvalue_2 (`KismetMaterialLibrary.CreateDynamicMaterialInstance` "/Game/Texture/M_Bllood.M_Bllood"))
      (set `self.Mt_blood` _returnvalue_2))
    (:`then_1`
      (bind _returnvalue_3 (`ColorFunctionLibrary.DuplicateRenderTarget` (`self.originTextureRenderTarget`)))
      (set `self.new_TextureRenderTarget` _returnvalue_3)
      (bind _returnvalue_4 (`ColorFunctionLibrary.DuplicateRenderTarget` (`self.originPercent Render Target`)))
      (set `self.new_Percent Render Target` _returnvalue_4))
    (:`then_2`
      (`MaterialInstanceDynamic.SetTextureParameterValue` (`self.Mt_blood`) "Param" (`self.new_Percent Render Target`)))
    (:`then_3`
      (bind _returnvalue_5 (`KismetMaterialLibrary.CreateDynamicMaterialInstance` "/Game/Texture/M_BlloodCalc.M_BlloodCalc"))
      (set `self.Mt_bloodCalc` _returnvalue_5))))

(event `CleanPaint`
  (params (playerArea :type "Vector Structure"))
  (bind (_nextuv_x _nextuv_y) (`KismetMathLibrary.BreakVector` (`self.nextUV`)))
  (`self.Draw Area` playerArea)
  (`MaterialInstanceDynamic.SetVectorParameterValue` (`self.dartMat`) "Area" (make `LinearColor` _nextuv_x _nextuv_y))
  (`KismetRenderingLibrary.DrawMaterialToRenderTarget` (`self.new_TextureRenderTarget`) (`self.dartMat`))
  (`self.CheckCleanPer`))

(event `printTex`
  (bind (_nextuv_x _nextuv_y) (`KismetMathLibrary.BreakVector` (`self.nextUV`)))
  (`KismetRenderingLibrary.DrawMaterialToRenderTarget` (`self.new_TextureRenderTarget`) (`self.dartMat`))
  (`MaterialInstanceDynamic.SetVectorParameterValue` (`self.dartMat`) "Area" (make `LinearColor` _nextuv_x _nextuv_y)))

(fn `CheckCleanPer`
  (`|ExecutionSequence`
    (:`then_0`
      (`KismetRenderingLibrary.DrawMaterialToRenderTarget` (`self.new_Percent Render Target`) (`self.Mt_bloodCalc`)))
    (:`then_1`
      (bind _returnvalue (`ColorFunctionLibrary.GetCleaningRate` (`self.new_Percent Render Target`)))
      (`KismetSystemLibrary.PrintText` (`KismetTextLibrary.Conv_DoubleToText` (* _returnvalue 100.0) "HalfToEven")))))

(fn `Draw Area`
  (params (playerLocation :type "Vector Structure"))
  (locals (location :type "Vector Structure" :default (0.0 0.0 0.0)) (width :type "Float (double-precision)") (height :type "Float (double-precision)") (boxExtent :type "Vector Structure" :default (0.0 0.0 0.0)))
  (bind (_boxextent_x _boxextent_y) (`KismetMathLibrary.BreakVector` (`local.boxExtent`)))
  (bind _boxextent_x_2 (`KismetMathLibrary.BreakVector` (`local.boxExtent`)))
  (bind _location_x (`KismetMathLibrary.BreakVector` (`local.location`)))
  (bind (_location_x_2 _location_y) (`KismetMathLibrary.BreakVector` (`local.location`)))
  (bind _location_x_3 (`KismetMathLibrary.BreakVector` (`local.location`)))
  (bind (_location_x_4 _location_y_2) (`KismetMathLibrary.BreakVector` (`local.location`)))
  (bind (_returnvalue_x _returnvalue_y) (`KismetMathLibrary.BreakVector` (`SceneComponent.K2_GetComponentScale` (`self.Plane`))))
  (bind _returnvalue_x_2 (`KismetMathLibrary.BreakVector` (`SceneComponent.K2_GetComponentScale` (`self.Plane`))))
  (`|ExecutionSequence`
    (:`then_0`
      (set `local.location` (`KismetMathLibrary.InverseTransformLocation` (`self.GetTransform`) (`local.playerLocation`)))
      (set `local.boxExtent` (`.BoxExtent` (`KismetMathLibrary.BreakBoxSphereBounds` (`StaticMesh.GetBounds` (`StaticMeshComponent.StaticMesh` (`self.Plane`)))))))
    (:`then_1`
      (set `local.width` (* _boxextent_x_2 _returnvalue_x_2 2.0))
      (set `local.height` (* _boxextent_y _returnvalue_y 2.0)))
    (:`then_2`
      (if (and (<= (`KismetMathLibrary.Abs` _location_x) (/ (`local.width`) 2.0)) (<= (`KismetMathLibrary.Abs` _location_y_2) (/ (`local.height`) 2.0)))
        (set `self.nextUV` (`KismetMathLibrary.MakeVector` (+ (/ _location_x_3 (`local.width`)) 0.5) (+ (/ _location_y (`local.height`)) 0.5)))
        (else
          (set `self.nextUV` (-1.0 -1.0 0.0)))))))

(fn `UserConstructionScript`)