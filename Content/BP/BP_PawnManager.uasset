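; BP_PawnManager spawns and keeps track of BP_ClonePawn clones, adding one each time the AddNewChara event fires.
; AddNewClone offsets each spawn along negative X by the current list length, so clones line up at even intervals.
; Each clone attaches to the manager's root with relative rules, joins SkeltalMeshList, then has Run called on it.
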(event `AddNewChara`
  (`self.Add New Clone`))

(fn `Add New Clone`
  (locals (tmpClone :type "/Game/BP/BP_ClonePawn Object Reference"))
  (`|ExecutionSequence`
    (:`then_0`
      (bind _returnvalue (`|SpawnActorFromClass` "/Game/BP/BP_ClonePawn.BP_ClonePawn_C" (`KismetMathLibrary.MakeTransform` (`KismetMathLibrary.MakeVector` (`KismetMathLibrary.Conv_IntToDouble` (* (`KismetArrayLibrary.Array_Length` (`self.SkeltalMeshList`)) -100)))) "Undefined" "MultiplyWithRoot" null null))
      (bind _output_get (set `local.tmpClone` _returnvalue))
      (`self.K2_AttachToComponent` _output_get (`self.DefaultSceneRoot`) "None" "KeepRelative" "KeepRelative" "KeepRelative" true)
      (`KismetArrayLibrary.Array_Add` (`self.SkeltalMeshList`) (`local.tmpClone`)))
    (:`then_1`
      (`/Game/BP/BP_ClonePawn.Run` (`local.tmpClone`)))))

(fn `UserConstructionScript`)